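; Embers actor that prints screen-space annotations (class, ID, center, bounding-box size) for Niagara ember particles, alongside a per-tick frame counter.
; Niagara exports particles to ParticleData, with Size carrying ID and Velocity carrying mesh size, whose box corners are projected through the player camera.
; A looping timer applies settings.txt temperature and intensity lines to directional lights, quitting once the line index exceeds three.
; Fire-bounds and log-saving nodes are disconnected.
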(event Custom|ProcessNextLine
  ;[1 1 1] read settings from file and and split lines
  (bind _returnvalue (Class|Readdata|LoadFiletoString "settings.txt"))
  (bind _outactors (Actor|GetAllActorsOfClass "/Script/Engine.DirectionalLight"))
  (for _array_element _outactors
    (Class|LightComponent|SetTemperature (Variables|/Script/Engine.Light|GetLightComponent _array_element) (Math|Conversions|ToFloat(Integer) (Utilities|Array|Get(acopy) (Utilities|String|ParseIntoArray (Utilities|Array|Get(acopy) (Utilities|String|ParseIntoArray _returnvalue "  
") (Variables|Default|GetCurrentLineIndex)) ","))))
    (Rendering|Components|Light|SetIntensity (Variables|/Script/Engine.Light|GetLightComponent _array_element) (Math|Conversions|ToFloat(Integer) (Utilities|Array|Get(acopy) (Utilities|String|ParseIntoArray (Utilities|Array|Get(acopy) (Utilities|String|ParseIntoArray _returnvalue "  
") (Variables|Default|GetCurrentLineIndex)) ",") 1)))
    (bind _result (Math|Integer|IncrementInt (Variables|Default|GetCurrentLineIndex))
      (:%20%20
        (bind _output_get (Variables|Default|SetCurrentLineIndex _result))
        (if (> _output_get 3)
          (Development|ExecuteConsoleCommand "quit" 0))))))

(event EventBeginPlay
  ;[1 1 1] data send to call back
  (Niagara|SetNiagaraVariable(Object) (Variables|Default|GetNiagara) "user.BPcallback" self) ; every timed start game we going to export the data to the bp call back parameter(blueprint)
  (Utilities|Time|SetTimerbyFunctionName 0 "ProcessNextLine" 2e+01 true))

(event EventTick
  (params (DeltaSeconds :type Float%20%28single-precision%29))
  (bind _result (Math|Integer|IncrementInt (Variables|Default|GetNewVar_0))
    (:%20%20
      (Development|PrintString (Utilities|String|Append "Frame: " (Utilities|String|ToString(Integer) _result)) true true "(R=1.000000,G=0.054835,B=0.969464,A=1.000000)"))))

(event EventParticleData
  (params (Data :type Array%20of%20Basic%20Particle%20Data%20Structures) (NiagaraSystem :type Niagara%20System%20Object%20Reference))
  (bind _returnvalue (Game|GetPlayerController 0))
  ;[1 1 1] Receive and Handle Particle Data from Niagara System
  (for _array_element Data
    (Development|PrintString "CLASS: Embers")
    (Development|PrintString (Utilities|String|Append "ID: " (Utilities|String|ToString(Float) (.Size (Utilities|Struct|BreakBasicParticleData _array_element)))))
    (Development|PrintString (Utilities|String|Append "Center: " (Utilities|String|ToString(Vector2d) (.ScreenLocation (Class|PlayerController|ProjectWorldLocationtoScreen _returnvalue (.Position (Utilities|Struct|BreakBasicParticleData _array_element)) true)))) true true "(R=1.000000,G=0.901327,B=0.068713,A=1.000000)")
    (Development|PrintString (Utilities|String|Append "BBOX: " (Utilities|String|ToString(Vector2d) (Math|Vector2D|MakeVector2D (- (Math|Float|Max(Float) (.X (Math|Vector2D|BreakVector2D (.ScreenLocation (Class|PlayerController|ProjectWorldLocationtoScreen _returnvalue (+ (.Position (Utilities|Struct|BreakBasicParticleData _array_element)) (/ (.Velocity (Utilities|Struct|BreakBasicParticleData _array_element)) 2)) true)))) (.X (Math|Vector2D|BreakVector2D (.ScreenLocation (Class|PlayerController|ProjectWorldLocationtoScreen _returnvalue (- (.Position (Utilities|Struct|BreakBasicParticleData _array_element)) (/ (.Velocity (Utilities|Struct|BreakBasicParticleData _array_element)) 2)) true)))) (.X (Math|Vector2D|BreakVector2D (.ScreenLocation (Class|PlayerController|ProjectWorldLocationtoScreen _returnvalue (Math|Vector|MakeVector (+ (.X (Math|Vector|BreakVector (.Position (Utilities|Struct|BreakBasicParticleData _array_element)))) (.X (Math|Vector|BreakVector (/ (.Velocity (Utilities|Struct|BreakBasicParticleData _array_element)) 2)))) (+ (.Y (Math|Vector|BreakVector (.Position (Utilities|Struct|BreakBasicParticleData _array_element)))) (.Y (Math|Vector|BreakVector (/ (.Velocity (Utilities|Struct|BreakBasicParticleData _array_element)) 2)))) (- (.Z (Math|Vector|BreakVector (.Position (Utilities|Struct|BreakBasicParticleData _array_element)))) (.Z (Math|Vector|BreakVector (/ (.Velocity (Utilities|Struct|BreakBasicParticleData _array_element)) 2))))) true)))) (.X (Math|Vector2D|BreakVector2D (.ScreenLocation (Class|PlayerController|ProjectWorldLocationtoScreen _returnvalue (Math|Vector|MakeVector (+ (.X (Math|Vector|BreakVector (.Position (Utilities|Struct|BreakBasicParticleData _array_element)))) (.X (Math|Vector|BreakVector (/ (.Velocity (Utilities|Struct|BreakBasicParticleData _array_element)) 2)))) (- (.Y (Math|Vector|BreakVector (.Position (Utilities|Struct|BreakBasicParticleData _array_element)))) (.Y (Math|Vector|BreakVector (/ (.Velocity (Utilities|Struct|BreakBasicParticleData _array_element)) 2)))) (+ (.Z (Math|Vector|BreakVector (.Position (Utilities|Struct|BreakBasicParticleData _array_element)))) (.Z (Math|Vector|BreakVector (/ (.Velocity (Utilities|Struct|BreakBasicParticleData _array_element)) 2))))) true)))) (.X (Math|Vector2D|BreakVector2D (.ScreenLocation (Class|PlayerController|ProjectWorldLocationtoScreen _returnvalue (Math|Vector|MakeVector (+ (.X (Math|Vector|BreakVector (.Position (Utilities|Struct|BreakBasicParticleData _array_element)))) (.X (Math|Vector|BreakVector (/ (.Velocity (Utilities|Struct|BreakBasicParticleData _array_element)) 2)))) (- (.Y (Math|Vector|BreakVector (.Position (Utilities|Struct|BreakBasicParticleData _array_element)))) (.Y (Math|Vector|BreakVector (/ (.Velocity (Utilities|Struct|BreakBasicParticleData _array_element)) 2)))) (- (.Z (Math|Vector|BreakVector (.Position (Utilities|Struct|BreakBasicParticleData _array_element)))) (.Z (Math|Vector|BreakVector (/ (.Velocity (Utilities|Struct|BreakBasicParticleData _array_element)) 2))))) true)))) (.X (Math|Vector2D|BreakVector2D (.ScreenLocation (Class|PlayerController|ProjectWorldLocationtoScreen _returnvalue (Math|Vector|MakeVector (- (.X (Math|Vector|BreakVector (.Position (Utilities|Struct|BreakBasicParticleData _array_element)))) (.X (Math|Vector|BreakVector (/ (.Velocity (Utilities|Struct|BreakBasicParticleData _array_element)) 2)))) (+ (.Y (Math|Vector|BreakVector (.Position (Utilities|Struct|BreakBasicParticleData _array_element)))) (.Y (Math|Vector|BreakVector (/ (.Velocity (Utilities|Struct|BreakBasicParticleData _array_element)) 2)))) (+ (.Z (Math|Vector|BreakVector (.Position (Utilities|Struct|BreakBasicParticleData _array_element)))) (.Z (Math|Vector|BreakVector (/ (.Velocity (Utilities|Struct|BreakBasicParticleData _array_element)) 2))))) true)))) (.X (Math|Vector2D|BreakVector2D (.ScreenLocation (Class|PlayerController|ProjectWorldLocationtoScreen _returnvalue (Math|Vector|MakeVector (- (.X (Math|Vector|BreakVector (.Position (Utilities|Struct|BreakBasicParticleData _array_element)))) (.X (Math|Vector|BreakVector (/ (.Velocity (Utilities|Struct|BreakBasicParticleData _array_element)) 2)))) (+ (.Y (Math|Vector|BreakVector (.Position (Utilities|Struct|BreakBasicParticleData _array_element)))) (.Y (Math|Vector|BreakVector (/ (.Velocity (Utilities|Struct|BreakBasicParticleData _array_element)) 2)))) (- (.Z (Math|Vector|BreakVector (.Position (Utilities|Struct|BreakBasicParticleData _array_element)))) (.Z (Math|Vector|BreakVector (/ (.Velocity (Utilities|Struct|BreakBasicParticleData _array_element)) 2))))) true)))) (.X (Math|Vector2D|BreakVector2D (.ScreenLocation (Class|PlayerController|ProjectWorldLocationtoScreen _returnvalue (Math|Vector|MakeVector (- (.X (Math|Vector|BreakVector (.Position (Utilities|Struct|BreakBasicParticleData _array_element)))) (.X (Math|Vector|BreakVector (/ (.Velocity (Utilities|Struct|BreakBasicParticleData _array_element)) 2)))) (- (.Y (Math|Vector|BreakVector (.Position (Utilities|Struct|BreakBasicParticleData _array_element)))) (.Y (Math|Vector|BreakVector (/ (.Velocity (Utilities|Struct|BreakBasicParticleData _array_element)) 2)))) (+ (.Z (Math|Vector|BreakVector (.Position (Utilities|Struct|BreakBasicParticleData _array_element)))) (.Z (Math|Vector|BreakVector (/ (.Velocity (Utilities|Struct|BreakBasicParticleData _array_element)) 2))))) true))))) (Math|Float|Min(Float) (.X (Math|Vector2D|BreakVector2D (.ScreenLocation (Class|PlayerController|ProjectWorldLocationtoScreen _returnvalue (+ (.Position (Utilities|Struct|BreakBasicParticleData _array_element)) (/ (.Velocity (Utilities|Struct|BreakBasicParticleData _array_element)) 2)) true)))) (.X (Math|Vector2D|BreakVector2D (.ScreenLocation (Class|PlayerController|ProjectWorldLocationtoScreen _returnvalue (- (.Position (Utilities|Struct|BreakBasicParticleData _array_element)) (/ (.Velocity (Utilities|Struct|BreakBasicParticleData _array_element)) 2)) true)))) (.X (Math|Vector2D|BreakVector2D (.ScreenLocation (Class|PlayerController|ProjectWorldLocationtoScreen _returnvalue (Math|Vector|MakeVector (+ (.X (Math|Vector|BreakVector (.Position (Utilities|Struct|BreakBasicParticleData _array_element)))) (.X (Math|Vector|BreakVector (/ (.Velocity (Utilities|Struct|BreakBasicParticleData _array_element)) 2)))) (+ (.Y (Math|Vector|BreakVector (.Position (Utilities|Struct|BreakBasicParticleData _array_element)))) (.Y (Math|Vector|BreakVector (/ (.Velocity (Utilities|Struct|BreakBasicParticleData _array_element)) 2)))) (- (.Z (Math|Vector|BreakVector (.Position (Utilities|Struct|BreakBasicParticleData _array_element)))) (.Z (Math|Vector|BreakVector (/ (.Velocity (Utilities|Struct|BreakBasicParticleData _array_element)) 2))))) true)))) (.X (Math|Vector2D|BreakVector2D (.ScreenLocation (Class|PlayerController|ProjectWorldLocationtoScreen _returnvalue (Math|Vector|MakeVector (+ (.X (Math|Vector|BreakVector (.Position (Utilities|Struct|BreakBasicParticleData _array_element)))) (.X (Math|Vector|BreakVector (/ (.Velocity (Utilities|Struct|BreakBasicParticleData _array_element)) 2)))) (- (.Y (Math|Vector|BreakVector (.Position (Utilities|Struct|BreakBasicParticleData _array_element)))) (.Y (Math|Vector|BreakVector (/ (.Velocity (Utilities|Struct|BreakBasicParticleData _array_element)) 2)))) (+ (.Z (Math|Vector|BreakVector (.Position (Utilities|Struct|BreakBasicParticleData _array_element)))) (.Z (Math|Vector|BreakVector (/ (.Velocity (Utilities|Struct|BreakBasicParticleData _array_element)) 2))))) true)))) (.X (Math|Vector2D|BreakVector2D (.ScreenLocation (Class|PlayerController|ProjectWorldLocationtoScreen _returnvalue (Math|Vector|MakeVector (+ (.X (Math|Vector|BreakVector (.Position (Utilities|Struct|BreakBasicParticleData _array_element)))) (.X (Math|Vector|BreakVector (/ (.Velocity (Utilities|Struct|BreakBasicParticleData _array_element)) 2)))) (- (.Y (Math|Vector|BreakVector (.Position (Utilities|Struct|BreakBasicParticleData _array_element)))) (.Y (Math|Vector|BreakVector (/ (.Velocity (Utilities|Struct|BreakBasicParticleData _array_element)) 2)))) (- (.Z (Math|Vector|BreakVector (.Position (Utilities|Struct|BreakBasicParticleData _array_element)))) (.Z (Math|Vector|BreakVector (/ (.Velocity (Utilities|Struct|BreakBasicParticleData _array_element)) 2))))) true)))) (.X (Math|Vector2D|BreakVector2D (.ScreenLocation (Class|PlayerController|ProjectWorldLocationtoScreen _returnvalue (Math|Vector|MakeVector (- (.X (Math|Vector|BreakVector (.Position (Utilities|Struct|BreakBasicParticleData _array_element)))) (.X (Math|Vector|BreakVector (/ (.Velocity (Utilities|Struct|BreakBasicParticleData _array_element)) 2)))) (+ (.Y (Math|Vector|BreakVector (.Position (Utilities|Struct|BreakBasicParticleData _array_element)))) (.Y (Math|Vector|BreakVector (/ (.Velocity (Utilities|Struct|BreakBasicParticleData _array_element)) 2)))) (+ (.Z (Math|Vector|BreakVector (.Position (Utilities|Struct|BreakBasicParticleData _array_element)))) (.Z (Math|Vector|BreakVector (/ (.Velocity (Utilities|Struct|BreakBasicParticleData _array_element)) 2))))) true)))) (.X (Math|Vector2D|BreakVector2D (.ScreenLocation (Class|PlayerController|ProjectWorldLocationtoScreen _returnvalue (Math|Vector|MakeVector (- (.X (Math|Vector|BreakVector (.Position (Utilities|Struct|BreakBasicParticleData _array_element)))) (.X (Math|Vector|BreakVector (/ (.Velocity (Utilities|Struct|BreakBasicParticleData _array_element)) 2)))) (+ (.Y (Math|Vector|BreakVector (.Position (Utilities|Struct|BreakBasicParticleData _array_element)))) (.Y (Math|Vector|BreakVector (/ (.Velocity (Utilities|Struct|BreakBasicParticleData _array_element)) 2)))) (- (.Z (Math|Vector|BreakVector (.Position (Utilities|Struct|BreakBasicParticleData _array_element)))) (.Z (Math|Vector|BreakVector (/ (.Velocity (Utilities|Struct|BreakBasicParticleData _array_element)) 2))))) true)))) (.X (Math|Vector2D|BreakVector2D (.ScreenLocation (Class|PlayerController|ProjectWorldLocationtoScreen _returnvalue (Math|Vector|MakeVector (- (.X (Math|Vector|BreakVector (.Position (Utilities|Struct|BreakBasicParticleData _array_element)))) (.X (Math|Vector|BreakVector (/ (.Velocity (Utilities|Struct|BreakBasicParticleData _array_element)) 2)))) (- (.Y (Math|Vector|BreakVector (.Position (Utilities|Struct|BreakBasicParticleData _array_element)))) (.Y (Math|Vector|BreakVector (/ (.Velocity (Utilities|Struct|BreakBasicParticleData _array_element)) 2)))) (+ (.Z (Math|Vector|BreakVector (.Position (Utilities|Struct|BreakBasicParticleData _array_element)))) (.Z (Math|Vector|BreakVector (/ (.Velocity (Utilities|Struct|BreakBasicParticleData _array_element)) 2))))) true)))))) (- (Math|Float|Max(Float) (.Y (Math|Vector2D|BreakVector2D (.ScreenLocation (Class|PlayerController|ProjectWorldLocationtoScreen _returnvalue (+ (.Position (Utilities|Struct|BreakBasicParticleData _array_element)) (/ (.Velocity (Utilities|Struct|BreakBasicParticleData _array_element)) 2)) true)))) (.Y (Math|Vector2D|BreakVector2D (.ScreenLocation (Class|PlayerController|ProjectWorldLocationtoScreen _returnvalue (- (.Position (Utilities|Struct|BreakBasicParticleData _array_element)) (/ (.Velocity (Utilities|Struct|BreakBasicParticleData _array_element)) 2)) true)))) (.Y (Math|Vector2D|BreakVector2D (.ScreenLocation (Class|PlayerController|ProjectWorldLocationtoScreen _returnvalue (Math|Vector|MakeVector (+ (.X (Math|Vector|BreakVector (.Position (Utilities|Struct|BreakBasicParticleData _array_element)))) (.X (Math|Vector|BreakVector (/ (.Velocity (Utilities|Struct|BreakBasicParticleData _array_element)) 2)))) (+ (.Y (Math|Vector|BreakVector (.Position (Utilities|Struct|BreakBasicParticleData _array_element)))) (.Y (Math|Vector|BreakVector (/ (.Velocity (Utilities|Struct|BreakBasicParticleData _array_element)) 2)))) (- (.Z (Math|Vector|BreakVector (.Position (Utilities|Struct|BreakBasicParticleData _array_element)))) (.Z (Math|Vector|BreakVector (/ (.Velocity (Utilities|Struct|BreakBasicParticleData _array_element)) 2))))) true)))) (.Y (Math|Vector2D|BreakVector2D (.ScreenLocation (Class|PlayerController|ProjectWorldLocationtoScreen _returnvalue (Math|Vector|MakeVector (+ (.X (Math|Vector|BreakVector (.Position (Utilities|Struct|BreakBasicParticleData _array_element)))) (.X (Math|Vector|BreakVector (/ (.Velocity (Utilities|Struct|BreakBasicParticleData _array_element)) 2)))) (- (.Y (Math|Vector|BreakVector (.Position (Utilities|Struct|BreakBasicParticleData _array_element)))) (.Y (Math|Vector|BreakVector (/ (.Velocity (Utilities|Struct|BreakBasicParticleData _array_element)) 2)))) (+ (.Z (Math|Vector|BreakVector (.Position (Utilities|Struct|BreakBasicParticleData _array_element)))) (.Z (Math|Vector|BreakVector (/ (.Velocity (Utilities|Struct|BreakBasicParticleData _array_element)) 2))))) true)))) (.Y (Math|Vector2D|BreakVector2D (.ScreenLocation (Class|PlayerController|ProjectWorldLocationtoScreen _returnvalue (Math|Vector|MakeVector (+ (.X (Math|Vector|BreakVector (.Position (Utilities|Struct|BreakBasicParticleData _array_element)))) (.X (Math|Vector|BreakVector (/ (.Velocity (Utilities|Struct|BreakBasicParticleData _array_element)) 2)))) (- (.Y (Math|Vector|BreakVector (.Position (Utilities|Struct|BreakBasicParticleData _array_element)))) (.Y (Math|Vector|BreakVector (/ (.Velocity (Utilities|Struct|BreakBasicParticleData _array_element)) 2)))) (- (.Z (Math|Vector|BreakVector (.Position (Utilities|Struct|BreakBasicParticleData _array_element)))) (.Z (Math|Vector|BreakVector (/ (.Velocity (Utilities|Struct|BreakBasicParticleData _array_element)) 2))))) true)))) (.Y (Math|Vector2D|BreakVector2D (.ScreenLocation (Class|PlayerController|ProjectWorldLocationtoScreen _returnvalue (Math|Vector|MakeVector (- (.X (Math|Vector|BreakVector (.Position (Utilities|Struct|BreakBasicParticleData _array_element)))) (.X (Math|Vector|BreakVector (/ (.Velocity (Utilities|Struct|BreakBasicParticleData _array_element)) 2)))) (+ (.Y (Math|Vector|BreakVector (.Position (Utilities|Struct|BreakBasicParticleData _array_element)))) (.Y (Math|Vector|BreakVector (/ (.Velocity (Utilities|Struct|BreakBasicParticleData _array_element)) 2)))) (+ (.Z (Math|Vector|BreakVector (.Position (Utilities|Struct|BreakBasicParticleData _array_element)))) (.Z (Math|Vector|BreakVector (/ (.Velocity (Utilities|Struct|BreakBasicParticleData _array_element)) 2))))) true)))) (.Y (Math|Vector2D|BreakVector2D (.ScreenLocation (Class|PlayerController|ProjectWorldLocationtoScreen _returnvalue (Math|Vector|MakeVector (- (.X (Math|Vector|BreakVector (.Position (Utilities|Struct|BreakBasicParticleData _array_element)))) (.X (Math|Vector|BreakVector (/ (.Velocity (Utilities|Struct|BreakBasicParticleData _array_element)) 2)))) (+ (.Y (Math|Vector|BreakVector (.Position (Utilities|Struct|BreakBasicParticleData _array_element)))) (.Y (Math|Vector|BreakVector (/ (.Velocity (Utilities|Struct|BreakBasicParticleData _array_element)) 2)))) (- (.Z (Math|Vector|BreakVector (.Position (Utilities|Struct|BreakBasicParticleData _array_element)))) (.Z (Math|Vector|BreakVector (/ (.Velocity (Utilities|Struct|BreakBasicParticleData _array_element)) 2))))) true)))) (.Y (Math|Vector2D|BreakVector2D (.ScreenLocation (Class|PlayerController|ProjectWorldLocationtoScreen _returnvalue (Math|Vector|MakeVector (- (.X (Math|Vector|BreakVector (.Position (Utilities|Struct|BreakBasicParticleData _array_element)))) (.X (Math|Vector|BreakVector (/ (.Velocity (Utilities|Struct|BreakBasicParticleData _array_element)) 2)))) (- (.Y (Math|Vector|BreakVector (.Position (Utilities|Struct|BreakBasicParticleData _array_element)))) (.Y (Math|Vector|BreakVector (/ (.Velocity (Utilities|Struct|BreakBasicParticleData _array_element)) 2)))) (+ (.Z (Math|Vector|BreakVector (.Position (Utilities|Struct|BreakBasicParticleData _array_element)))) (.Z (Math|Vector|BreakVector (/ (.Velocity (Utilities|Struct|BreakBasicParticleData _array_element)) 2))))) true))))) (Math|Float|Min(Float) (.Y (Math|Vector2D|BreakVector2D (.ScreenLocation (Class|PlayerController|ProjectWorldLocationtoScreen _returnvalue (+ (.Position (Utilities|Struct|BreakBasicParticleData _array_element)) (/ (.Velocity (Utilities|Struct|BreakBasicParticleData _array_element)) 2)) true)))) (.Y (Math|Vector2D|BreakVector2D (.ScreenLocation (Class|PlayerController|ProjectWorldLocationtoScreen _returnvalue (- (.Position (Utilities|Struct|BreakBasicParticleData _array_element)) (/ (.Velocity (Utilities|Struct|BreakBasicParticleData _array_element)) 2)) true)))) (.Y (Math|Vector2D|BreakVector2D (.ScreenLocation (Class|PlayerController|ProjectWorldLocationtoScreen _returnvalue (Math|Vector|MakeVector (+ (.X (Math|Vector|BreakVector (.Position (Utilities|Struct|BreakBasicParticleData _array_element)))) (.X (Math|Vector|BreakVector (/ (.Velocity (Utilities|Struct|BreakBasicParticleData _array_element)) 2)))) (+ (.Y (Math|Vector|BreakVector (.Position (Utilities|Struct|BreakBasicParticleData _array_element)))) (.Y (Math|Vector|BreakVector (/ (.Velocity (Utilities|Struct|BreakBasicParticleData _array_element)) 2)))) (- (.Z (Math|Vector|BreakVector (.Position (Utilities|Struct|BreakBasicParticleData _array_element)))) (.Z (Math|Vector|BreakVector (/ (.Velocity (Utilities|Struct|BreakBasicParticleData _array_element)) 2))))) true)))) (.Y (Math|Vector2D|BreakVector2D (.ScreenLocation (Class|PlayerController|ProjectWorldLocationtoScreen _returnvalue (Math|Vector|MakeVector (+ (.X (Math|Vector|BreakVector (.Position (Utilities|Struct|BreakBasicParticleData _array_element)))) (.X (Math|Vector|BreakVector (/ (.Velocity (Utilities|Struct|BreakBasicParticleData _array_element)) 2)))) (- (.Y (Math|Vector|BreakVector (.Position (Utilities|Struct|BreakBasicParticleData _array_element)))) (.Y (Math|Vector|BreakVector (/ (.Velocity (Utilities|Struct|BreakBasicParticleData _array_element)) 2)))) (+ (.Z (Math|Vector|BreakVector (.Position (Utilities|Struct|BreakBasicParticleData _array_element)))) (.Z (Math|Vector|BreakVector (/ (.Velocity (Utilities|Struct|BreakBasicParticleData _array_element)) 2))))) true)))) (.Y (Math|Vector2D|BreakVector2D (.ScreenLocation (Class|PlayerController|ProjectWorldLocationtoScreen _returnvalue (Math|Vector|MakeVector (+ (.X (Math|Vector|BreakVector (.Position (Utilities|Struct|BreakBasicParticleData _array_element)))) (.X (Math|Vector|BreakVector (/ (.Velocity (Utilities|Struct|BreakBasicParticleData _array_element)) 2)))) (- (.Y (Math|Vector|BreakVector (.Position (Utilities|Struct|BreakBasicParticleData _array_element)))) (.Y (Math|Vector|BreakVector (/ (.Velocity (Utilities|Struct|BreakBasicParticleData _array_element)) 2)))) (- (.Z (Math|Vector|BreakVector (.Position (Utilities|Struct|BreakBasicParticleData _array_element)))) (.Z (Math|Vector|BreakVector (/ (.Velocity (Utilities|Struct|BreakBasicParticleData _array_element)) 2))))) true)))) (.Y (Math|Vector2D|BreakVector2D (.ScreenLocation (Class|PlayerController|ProjectWorldLocationtoScreen _returnvalue (Math|Vector|MakeVector (- (.X (Math|Vector|BreakVector (.Position (Utilities|Struct|BreakBasicParticleData _array_element)))) (.X (Math|Vector|BreakVector (/ (.Velocity (Utilities|Struct|BreakBasicParticleData _array_element)) 2)))) (+ (.Y (Math|Vector|BreakVector (.Position (Utilities|Struct|BreakBasicParticleData _array_element)))) (.Y (Math|Vector|BreakVector (/ (.Velocity (Utilities|Struct|BreakBasicParticleData _array_element)) 2)))) (+ (.Z (Math|Vector|BreakVector (.Position (Utilities|Struct|BreakBasicParticleData _array_element)))) (.Z (Math|Vector|BreakVector (/ (.Velocity (Utilities|Struct|BreakBasicParticleData _array_element)) 2))))) true)))) (.Y (Math|Vector2D|BreakVector2D (.ScreenLocation (Class|PlayerController|ProjectWorldLocationtoScreen _returnvalue (Math|Vector|MakeVector (- (.X (Math|Vector|BreakVector (.Position (Utilities|Struct|BreakBasicParticleData _array_element)))) (.X (Math|Vector|BreakVector (/ (.Velocity (Utilities|Struct|BreakBasicParticleData _array_element)) 2)))) (+ (.Y (Math|Vector|BreakVector (.Position (Utilities|Struct|BreakBasicParticleData _array_element)))) (.Y (Math|Vector|BreakVector (/ (.Velocity (Utilities|Struct|BreakBasicParticleData _array_element)) 2)))) (- (.Z (Math|Vector|BreakVector (.Position (Utilities|Struct|BreakBasicParticleData _array_element)))) (.Z (Math|Vector|BreakVector (/ (.Velocity (Utilities|Struct|BreakBasicParticleData _array_element)) 2))))) true)))) (.Y (Math|Vector2D|BreakVector2D (.ScreenLocation (Class|PlayerController|ProjectWorldLocationtoScreen _returnvalue (Math|Vector|MakeVector (- (.X (Math|Vector|BreakVector (.Position (Utilities|Struct|BreakBasicParticleData _array_element)))) (.X (Math|Vector|BreakVector (/ (.Velocity (Utilities|Struct|BreakBasicParticleData _array_element)) 2)))) (- (.Y (Math|Vector|BreakVector (.Position (Utilities|Struct|BreakBasicParticleData _array_element)))) (.Y (Math|Vector|BreakVector (/ (.Velocity (Utilities|Struct|BreakBasicParticleData _array_element)) 2)))) (+ (.Z (Math|Vector|BreakVector (.Position (Utilities|Struct|BreakBasicParticleData _array_element)))) (.Z (Math|Vector|BreakVector (/ (.Velocity (Utilities|Struct|BreakBasicParticleData _array_element)) 2))))) true))))))))) true true "(R=0.129583,G=1.000000,B=0.000000,A=1.000000)")))

(fn ConstructionScript)