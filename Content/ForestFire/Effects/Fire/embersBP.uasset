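; Ember effect actor for the forest fire that reads individual particle data out of its Niagara system.
; On BeginPlay it passes itself as the user.singleember object, so Niagara delivers particle data to the ParticleData event.
; For each ember, it prints the position projected to player 0's screen, plus size and velocity, as debug output.
; An unconnected branch sketches saving the screen location to a save slot but never runs.
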(event EventBeginPlay
  ;[1 1 1] set to get Niagara system data
  (Niagara|SetNiagaraVariable(Object) (Variables|Default|GetNiagara) "user.singleember" self))

(event EventTick
  (params (DeltaSeconds :type Float%20%28single-precision%29)))

(event EventParticleData
  (params (Data :type Array%20of%20Basic%20Particle%20Data%20Structures) (NiagaraSystem :type Niagara%20System%20Object%20Reference))
  ;[1 1 1] Get Single Ember World Locations
  (for _array_element Data
    ;[1 1 1] Print to screen and log
    (Development|PrintString (Utilities|String|ToString(Vector2d) (.ScreenLocation (Class|PlayerController|ProjectWorldLocationtoScreen (Game|GetPlayerController 0) (.Position (Utilities|Struct|BreakBasicParticleData _array_element)) true))))
    (Development|PrintString (Utilities|String|ToString(Float) (.Size (Utilities|Struct|BreakBasicParticleData _array_element))) true true "(R=1.000000,G=0.000000,B=0.049691,A=1.000000)")
    (Development|PrintString (Utilities|String|ToString(Vector) (.Velocity (Utilities|Struct|BreakBasicParticleData _array_element))) true true "(R=0.086832,G=1.000000,B=0.123680,A=1.000000)")))

(fn ConstructionScript)